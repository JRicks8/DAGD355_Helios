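; FlareEnemy is a suicide-bomber enemy that chases the player and explodes, hurting the player and other enemies in its blast sphere.
; Each Tick traces to the player and, while sight is clear, chases, leaps by impulse at jumping range, or detonates up close.
; Death or a sufficiently large hit also triggers Explode, which spawns the effect and destroys the actor.
; The jump lockout counts down in frames, not seconds.
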(event `OnDeath`
  (`self.Explode`))

(event `self.ReceiveBeginPlay`
  (add `self.EnemyDied` (delegate `OnDeath`))
  (add `self.TakenDamage` (delegate `ExplodeOnDamage`))
  (set `self.Target` (`GameplayStatics.GetPlayerPawn` 0)))

(event `ExplodeOnDamage` :!signature `self.TakenDamage`
  (params (Damage :type "Float (double-precision)"))
  (if (>= Damage 15.0)
    (`self.Explode`)))

(event `self.ReceiveTick`
  (params (DeltaSeconds :type "Float (single-precision)"))
  (`parent.ReceiveTick` DeltaSeconds)
  ;[1 1 1] Update Jump
  (bind _result (`/Engine/EditorBlueprintResources/StandardMacros.DecrementInt` (`self.JumpDurationTimer`))
    (:`  `
      (if (<= _result 0)
        (set `self.Jumping` false)
        (else
          (set `self.Jumping` true)))
      ;[1 1 1] AI
      (bind _outhit (`self.LineTraceToTarget`))
      (cast `/Game/Blueprints/Player/playerCharacter` (`.HitActor` (`GameplayStatics.BreakHitResult` _outhit))
        (:`then`
          (set `self.CanSeePlayer` true)
          (if (<= (`self.DistanceToTarget`) (`self.ExplodingDistance`))
            (`self.Explode`)
            (elif (and (<= (`self.DistanceToTarget`) (`self.JumpingDistance`)) (not (`self.Jumping`)))
              (`self.JumpAtTarget`)
              (else
                (`|AIMoveTo` self (0.0 0.0 0.0) (`self.Target`) 0.0)))))
        (:`CastFailed`
          (set `self.CanSeePlayer` false))))))

(fn `Explode`
  (clear `self.TakenDamage`)
  (`NiagaraFunctionLibrary.SpawnSystemAtLocation` "/Game/Art/Effect/Big_Explosion_FX/FX_Big_Explosion.FX_Big_Explosion" (`self.K2_GetActorLocation`))
  (for _array_element (`PrimitiveComponent.GetOverlappingActors` (`self.ExplosionSphere`) null)
    (bind _asplayer_character (cast `/Game/Blueprints/Player/playerCharacter` _array_element)
      (:`then`
        (`/Game/Blueprints/Player/playerCharacter.TakeDamage` _asplayer_character 40))
      (:`CastFailed`
        (bind _asenemy_base (cast `/Game/Blueprints/Enemies/EnemyBase` _array_element))
        (if (!= _asenemy_base self)
          (`self.TakeDamage` _asenemy_base (`self.ExplosionDamage`) 0.0)))))
  (set `self.Health` 0.0)
  (`self.K2_DestroyActor`))

(fn `JumpAtTarget`
  (bind (_returnvalue_x _returnvalue_y) (`KismetMathLibrary.BreakVector` (* (`KismetMathLibrary.GetDirectionUnitVector` (`SceneComponent.K2_GetComponentLocation` (`self.CapsuleComponent`)) (`SceneComponent.K2_GetComponentLocation` (`Actor.RootComponent` (`self.Target`)))) (`self.JumpForce`))))
  (set `self.Jumping` true)
  (set `self.JumpDurationTimer` (`self.JumpDuration`))
  (`CharacterMovementComponent.AddImpulse` (`self.CharacterMovement`) (`KismetMathLibrary.MakeVector` _returnvalue_x _returnvalue_y 500.0) true))

(fn `LineTraceToTarget`
  (returns (OutHit :type "HitResult Structure") (ReturnValue :type Boolean))
  (bind _returnvalue (`SceneComponent.K2_GetComponentLocation` (`self.CapsuleComponent`)))
  (bind _returnvalue_2 (`SceneComponent.K2_GetComponentLocation` (`Actor.RootComponent` (`self.Target`))))
  (set `self.DistanceToTarget` (`KismetMathLibrary.Vector_Distance` _returnvalue _returnvalue_2))
  (bind (_outhit _returnvalue_3) (`KismetSystemLibrary.LineTraceSingle` _returnvalue _returnvalue_2 "TraceTypeQuery2"))
  (return _outhit _returnvalue_3))

(fn `UserConstructionScript`
  (`parent.UserConstructionScript`))